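; Openable door actor that swings open and closed in response to open and close requests from its OpenDoor component.
; It stores its initial rotation at BeginPlay, and the DoorSwing timeline adds a yaw OpenAngle to that rotation each update.
; Closing reverses the same timeline, and a Sound Timing event track plays the Doorlock sound at the door's location.
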(event OnCloseRequest(OpenDoor)
  (bind _openangle (Timeline|DoorSwing Reverse)
    (:Update
      (Transformation|SetActorRotation (Math|Rotator|CombineRotators (Variables|Default|GetInitialRotation) (Math|Rotator|MakeRotator 0.0 0.0 _openangle))))
    (:Sound_Timing
      (Audio|PlaySoundatLocation "/Game/Audio/door-lock.door-lock" (Transformation|GetActorLocation)))))

(event OnOpenRequest(OpenDoor)
  (bind _openangle (Timeline|DoorSwing Play)
    (:Update
      (Transformation|SetActorRotation (Math|Rotator|CombineRotators (Variables|Default|GetInitialRotation) (Math|Rotator|MakeRotator 0.0 0.0 _openangle))))
    (:Sound_Timing
      (Audio|PlaySoundatLocation "/Game/Audio/door-lock.door-lock" (Transformation|GetActorLocation)))))

(event EventBeginPlay
  (Variables|Default|SetInitialRotation (Transformation|GetActorRotation)))

(fn ConstructionScript)